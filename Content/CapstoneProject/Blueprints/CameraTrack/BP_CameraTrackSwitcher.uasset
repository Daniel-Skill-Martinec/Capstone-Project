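; BP_CameraTrackSwitcher is an overlap trigger that blends the player's view to its linked camera track while BP_ThirdPersonCharacter is inside it.
; Entering, or already overlapping one tick after BeginPlay, stores the character's current track and makes the character the linked track's cam owner.
; Exiting blends back to the stored track, or to the character if none exists, calling SetOwner rather than SetCamOwner on the linked track.
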(event `self.ReceiveBeginPlay`
  (bind _overlappingactors (`self.GetOverlappingActors` "/Game/CapstoneProject/Blueprints/BP_ThirdPersonCharacter.BP_ThirdPersonCharacter_C"))
  (`KismetSystemLibrary.DelayUntilNextTick`)
  (if (`KismetArrayLibrary.Array_IsNotEmpty` _overlappingactors)
    (bind _asbp_third_person_character (cast `/Game/CapstoneProject/Blueprints/BP_ThirdPersonCharacter` (`|GetArrayItem` _overlappingactors)))
    (`self.SwitchToLinkedCam` _asbp_third_person_character)))

(event `self.ReceiveActorBeginOverlap`
  (params (OtherActor :type "Actor Object Reference"))
  (bind _asbp_third_person_character (cast `/Game/CapstoneProject/Blueprints/BP_ThirdPersonCharacter` OtherActor))
  (`self.SwitchToLinkedCam` _asbp_third_person_character))

(event `self.ReceiveActorEndOverlap`
  (params (OtherActor :type "Actor Object Reference"))
  (bind _asbp_third_person_character (cast `/Game/CapstoneProject/Blueprints/BP_ThirdPersonCharacter` OtherActor))
  (`self.SwitchToOldCam` _asbp_third_person_character))

(fn `SwitchToLinkedCam`
  (params (Character :type "/Game/CapstoneProject/Blueprints/BP_ThirdPersonCharacter Object Reference") (`instant?` :type Boolean))
  (bind _character (`local.Character`))
  (set `self.OldTrack` (`/Game/CapstoneProject/Blueprints/BP_ThirdPersonCharacter.CameraTrack` _character))
  (bind _asplayer_controller (cast `PlayerController` (`Pawn.GetController` _character)))
  (`PlayerController.SetViewTargetWithBlend` _asplayer_controller (`self.LinkedTrack`) (`KismetMathLibrary.SelectFloat` 0.0 (`self.BlendTime`) (`local.instant?`)) "VTBlend_Cubic" 0.0 true)
  (bind _oldtrack (`self.OldTrack`)
    (:`then`
      (`/Game/CapstoneProject/Blueprints/CameraTrack/BP_CameraTrack.SetCamOwner` _oldtrack null))
    (:`else`
      _))
  (`/Game/CapstoneProject/Blueprints/CameraTrack/BP_CameraTrack.SetCamOwner` (`self.LinkedTrack`) (`local.Character`)))

(fn `SwitchToOldCam`
  (params (Character :type "/Game/CapstoneProject/Blueprints/BP_ThirdPersonCharacter Object Reference"))
  (bind _asplayer_controller (cast `PlayerController` (`Pawn.GetController` (`local.Character`))))
  (bind _oldtrack (`self.OldTrack`)
    (:`then`
      (`PlayerController.SetViewTargetWithBlend` _asplayer_controller _oldtrack (`self.BlendTime`) "VTBlend_Cubic" 0.0 false)
      (`self.SetOwner` (`self.LinkedTrack`) null)
      (`/Game/CapstoneProject/Blueprints/CameraTrack/BP_CameraTrack.SetCamOwner` (`self.OldTrack`) (`local.Character`))
      (set `self.OldTrack` null))
    (:`else`
      (`PlayerController.SetViewTargetWithBlend` _asplayer_controller (`local.Character`) (`self.BlendTime`) "VTBlend_Cubic" 0.0 false)
      (`self.SetOwner` (`self.LinkedTrack`) null))))

(fn `UserConstructionScript`)