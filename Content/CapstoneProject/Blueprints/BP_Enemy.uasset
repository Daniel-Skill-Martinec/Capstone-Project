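; BP_Enemy is an enemy character that chases the player and reacts to damage.
; On BeginPlay it starts an AI MoveTo toward the player character, re-issuing it shortly after each success, with no handling for failure.
; A similar Wonder loop roams to random reachable nearby points, but nothing in this Blueprint calls it.
; Damage reduces Health, knocking the enemy back and up, or enabling mesh physics simulation once Health is depleted.
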(event `self.ReceiveBeginPlay`
  (`self.Chase Player`))

(event `Chase Player`
  ;[1 1 1] Chase Player
  (`|AIMoveTo` self (0.0 0.0 0.0) (`GameplayStatics.GetPlayerCharacter` 0)
    (:`OnSuccess`
      (`KismetSystemLibrary.Delay` 0.2)
      (`self.Chase Player`))))

(event `Wonder`
  ;[1 1 1] Wonder System
  (`|AIMoveTo` self (`NavigationSystemV1.K2_GetRandomReachablePointInRadius` (`self.K2_GetActorLocation`) 500.0 null null) null
    (:`OnSuccess`
      (`KismetSystemLibrary.Delay` 0.2)
      (`self.Wonder`))))

(event `self.ReceiveAnyDamage`
  (params (Damage :type "Float (single-precision)") (DamageType :type "DamageType Object Reference") (InstigatedBy :type "Controller Object Reference") (DamageCauser :type "Actor Object Reference"))
  ;[1 1 1] Damage System
  (set `self.Health` (- (`self.Health`) Damage))
  (if (<= (`self.Health`) 0.0)
    (`PrimitiveComponent.SetSimulatePhysics` (`self.Mesh`) true)
    (else
      (`self.LaunchCharacter` (+ (* (`self.GetActorForwardVector`) -200.0) (* (`self.GetActorUpVector`) 100.0))))))

(fn `UserConstructionScript`)