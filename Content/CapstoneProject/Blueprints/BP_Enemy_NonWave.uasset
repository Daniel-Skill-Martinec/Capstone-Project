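; BP_Enemy_NonWave is a melee enemy character that chases the player from BeginPlay.
; On reaching the player it plays a push montage, whose notify sphere-traces for pawns to apply damage; completion restarts the chase.
; Damage plays a sound and knocks it backward, or at zero health ragdolls it before delayed destruction.
; A looping random-wander event exists but is never called, and sword-spawning logic is disconnected.
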(event `self.ReceiveBeginPlay`
  (`self.Chase Player`))

(event `Chase Player`
  (bind _attack_trace_pos (`self.Attack Trace Pos`))
  (bind _returnvalue (`SceneComponent.K2_GetComponentLocation` _attack_trace_pos))
  ;[1 1 1] Chase Player
  (`|AIMoveTo` self (0.0 0.0 0.0) (`GameplayStatics.GetPlayerCharacter` 0) 20.0
    (:`OnSuccess`
      (if (`self.CanAttack`)
        (`|PlayMontage` (`self.Mesh`) "/Game/Animation/Push_Montage.Push_Montage"
          (:`then`
            (set `self.CanAttack` false))
          (:`OnCompleted`
            (set `self.CanAttack` true)
            (`self.Chase Player`))
          (:`OnNotifyBegin`
            (bind (_outhit _returnvalue_2) (`KismetSystemLibrary.SphereTraceSingleForObjects` :`Start` _returnvalue :`End` (+ _returnvalue (* (`SceneComponent.GetForwardVector` _attack_trace_pos) 100.0)) :`Radius` 25.0 :`ObjectTypes` (`|MakeArray` "ObjectTypeQuery3" :!type "EObjectTypeQuery Enum") :`DrawDebugType` "ForDuration"))
            (if _returnvalue_2
              (`GameplayStatics.ApplyDamage` (`.HitActor` (`GameplayStatics.BreakHitResult` _outhit)) 10.0))))))))

(event `Wonder`
  ;[1 1 1] Wonder System
  (`|AIMoveTo` self (`NavigationSystemV1.K2_GetRandomReachablePointInRadius` (`self.K2_GetActorLocation`) 500.0 null null) null
    (:`OnSuccess`
      (`KismetSystemLibrary.Delay` 0.2)
      (`self.Wonder`))))

(event `self.ReceiveAnyDamage`
  (params (Damage :type "Float (single-precision)") (DamageType :type "DamageType Object Reference") (InstigatedBy :type "Controller Object Reference") (DamageCauser :type "Actor Object Reference"))
  ;[1 1 1] Damage System
  (set `self.Health` (- (`self.Health`) Damage))
  (`GameplayStatics.PlaySoundAtLocation` "/Game/Sounds/MS_Damage.MS_Damage" (`self.K2_GetActorLocation`) (struct) 1.0 1.0 0.0 null null null null)
  (if (<= (`self.Health`) 0.0)
    (`PrimitiveComponent.SetSimulatePhysics` (`self.Mesh`) true)
    (set `self.CanAttack` false)
    (`CharacterMovementComponent.DisableMovement` (`self.CharacterMovement`))
    (`KismetSystemLibrary.Delay` 5.0)
    (`self.K2_DestroyActor`)
    (else
      (`self.LaunchCharacter` (+ (* (`self.GetActorForwardVector`) -200.0) (* (`self.GetActorUpVector`) 100.0))))))

(fn `UserConstructionScript`)