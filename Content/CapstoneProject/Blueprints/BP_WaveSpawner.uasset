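; BP_WaveSpawner is a wave spawner actor that starts the first wave on BeginPlay and the next whenever no BP_Enemy actors remain.
; Tick passes through a short Delay to throttle the GetAllActorsOfClass check.
; SpawnWave plays the Wave_Complete sound, increments CurrentWave and reads that wave's spawn count from the Waves map values.
; All spawns use the spawner's own transform; random SpawnPositions selection and CheckForEnemies are unused.
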(event `self.ReceiveBeginPlay`
  (`self.Spawn Wave`))

(event `Spawn Wave`
  (`GameplayStatics.PlaySound2D` "/Game/Sounds/Wave_Complete.Wave_Complete" 1.0 1.0 0.0 null null)
  (`/Engine/EditorBlueprintResources/StandardMacros.IncrementInt` (`self.Current Wave`)
    (:`  `
      (bind _values (`BlueprintMapLibrary.Map_Values` (`self.Waves`)))
      (for _ (range 1 (+ (`|GetArrayItem` _values (- (`self.Current Wave`) 1)) 1))
        (`|SpawnActorFromClass` "/Game/CapstoneProject/Blueprints/BP_Enemy.BP_Enemy_C" (`self.GetTransform`) "AdjustIfPossibleButAlwaysSpawn" "MultiplyWithRoot" null null)))))

(event `self.ReceiveTick`
  (params (DeltaSeconds :type "Float (single-precision)"))
  (`KismetSystemLibrary.Delay` 0.2)
  (bind _outactors (`GameplayStatics.GetAllActorsOfClass` "/Game/CapstoneProject/Blueprints/BP_Enemy.BP_Enemy_C"))
  (if (== (`KismetArrayLibrary.Array_Length` _outactors) 0)
    (`self.Spawn Wave`)))

(event `Check For Enemies`)

(fn `UserConstructionScript`)